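; FairyGUI "Basics" demo that loads the package and shows a full-screen menu of UI feature samples with a back button.
; Clicked button names resolve to demo components, cached in a map and swapped into a container via controller c1.
; When the button gear animation stops, a per-demo Play function wires up that sample: popups, windows, drag-drop, depth sorting, pooled grids and others.
; Tick advances progress bars while that demo is on stage.
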(event `self.OnDemoStart`
  (bind _structout (setmembers `UIConfig` :`StructRef` (`FairyBlueprintLibrary.GetUIConfig`) :`ButtonSound` "ui://Basics/click" :`VerticalScrollBar` "ui://Basics/ScrollBar_VT" :`HorizontalScrollBar` "ui://Basics/ScrollBar_HZ" :`PopupMenu` "ui://Basics/PopupMenu"))
  (`FairyBlueprintLibrary.SetUIConfig` _structout)
  (`UIPackage.AddPackage` "/Game/UI/Basics.Basics")
  (bind _returnvalue (`UIPackage.CreateObject` "Basics" "Main" "/Script/FairyGUI.GComponent"))
  (bind _output_get (set `self.MainView` _returnvalue))
  (`GObject.SetParent` _output_get (`GRoot.Get`))
  (`GObject.MakeFullScreen` _output_get true)
  (set `self.Controller1` (`GComponent.GetController` _output_get "c1"))
  (set `self.DemoContainer` (`GComponent.GetChild` _output_get "container" "/Script/FairyGUI.GComponent"))
  (bind _output_get_2 (set `self.BackButton` (`GComponent.GetChild` _output_get "btn_Back" null)))
  (add `GObject.OnClick` _output_get_2 (delegate `Event ClickBack`))
  (`GObject.SetVisible` _output_get_2 false)
  (for _array_element (`self.DemoNames`)
    (add `GObject.OnClick` (`GComponent.GetChild` (`self.MainView`) (`KismetStringLibrary.Concat_StrStr` "btn_" _array_element) null) (`|CreateDelegate` :!event `Event ClickDemo`))))

(event `self.OnDemoEnd`
  (`UIPackage.RemovePackage` "Basics"))

(event `Event ClickBack`
  (params (EventContext :type "EventContext Object Reference"))
  (`GController.SetSelectedIndex` (`self.Controller1`) 0 true)
  (`GObject.SetVisible` (stale `self.OnDemoStart` _output_get_2) false))

(event `Event ClickDemo`
  (params (EventContext :type "EventContext Object Reference"))
  (bind _democontainer (`self.DemoContainer`))
  (bind (_value _returnvalue) (`BlueprintMapLibrary.Map_Find` (`self.DemoObjects`) (`self.DemoName`)))
  (set `self.DemoName` (`KismetStringLibrary.Concat_StrStr` "Demo_" (`KismetStringLibrary.GetSubstring` (`GObject.Name` (`EventContext.GetSender` EventContext)) 4 100)))
  (if _returnvalue
    (set `self.DemoObject` _value)
    (else
      (bind _returnvalue_2 (`UIPackage.CreateObject` "Basics" (`self.DemoName`) "/Script/FairyGUI.GComponent"))
      (bind _output_get (set `self.DemoObject` _returnvalue_2))
      (`BlueprintMapLibrary.Map_Add` (`self.DemoObjects`) (`self.DemoName`) _output_get)))
  (`GComponent.RemoveChildren` _democontainer 0 -1)
  (`GObject.SetParent` (`self.DemoObject`) _democontainer)
  (`GController.SetSelectedIndex` (`self.Controller1`) 1 true)
  (`GObject.SetVisible` (`self.BackButton`) true)
  (add `GObject.OnGearStop` (`GComponent.GetChild` (`self.MainView`) "btns" null) (delegate `Event Btns Animation Complete`)))

(event `Event PopupMenu`
  (params (EventContext :type "EventContext Object Reference"))
  (`/Engine/EditorBlueprintResources/StandardMacros.IsValid` (`self.PopupMenu`)
    (:`Is Valid`
      _)
    (:`Is Not Valid`
      (bind _returnvalue (`PopupMenu.CreatePopupMenu` ""))
      (bind _output_get (set `self.PopupMenu` _returnvalue))
      (`PopupMenu.AddItem` _output_get (`KismetTextLibrary.Conv_StringToText` "Item 1") (delegate `Event ClickMenu`))
      (`PopupMenu.AddItem` _output_get (`KismetTextLibrary.Conv_StringToText` "Item 2") (delegate `Event ClickMenu`))
      (`PopupMenu.AddItem` _output_get (`KismetTextLibrary.Conv_StringToText` "Item 3") (delegate `Event ClickMenu`))
      (`PopupMenu.AddItem` :`self` _output_get :`Caption` (`KismetTextLibrary.Conv_StringToText` "Item 4"))))
  (`PopupMenu.Show` (`self.PopupMenu`) (`EventContext.GetSender` EventContext) "Auto"))

(event `Event PopupPanel`
  (params (EventContext :type "EventContext Object Reference"))
  (if (not (`KismetSystemLibrary.IsValid` (`self.PopupPanel`)))
    (bind _returnvalue (`UIPackage.CreateObject` "Basics" "Component12" null))
    (set `self.PopupPanel` _returnvalue))
  (`GRoot.ShowPopup` (`GRoot.Get`) (`self.PopupPanel`) (`EventContext.GetSender` EventContext) "Auto"))

(event `Event ClickMenu`
  (params (EventContext :type "EventContext Object Reference"))
  (`KismetSystemLibrary.PrintString` (`KismetTextLibrary.Conv_TextToString` (`GObject.GetText` (`FairyBlueprintLibrary.GetVariantAsUObject` (`EventContext.GetData` EventContext) "/Script/FairyGUI.GObject")))))

(event `Event Btns Animation Complete`
  (params (EventContext :type "EventContext Object Reference"))
  (bind _demoobject (`self.DemoObject`))
  (bind _demoobject_2 (`self.DemoObject`))
  (bind _demoobject_3 (`self.DemoObject`))
  (bind _demoobject_4 (`self.DemoObject`))
  (bind _demoobject_5 (`self.DemoObject`))
  (bind _demoobject_6 (`self.DemoObject`))
  (bind _returnvalue (`GComponent.GetChild` _demoobject "list2" "/Script/FairyGUI.GList"))
  (bind _returnvalue_2 (`GComponent.GetChild` _demoobject "list1" "/Script/FairyGUI.GList"))
  (bind _returnvalue_3 (`GComponent.GetChild` (`self.ListItem`) "t2" "/Script/FairyGUI.GTextField"))
  (bind _returnvalue_4 (`GComponent.GetChild` (`self.ListItem`) "star" "/Script/FairyGUI.GProgressBar"))
  (bind _returnvalue_5 (`GComponent.GetChild` (`self.ListItem`) "t0" "/Script/FairyGUI.GObject"))
  (bind _returnvalue_6 (`GComponent.GetChild` (`self.ListItem`) "t1" "/Script/FairyGUI.GObject"))
  (bind _returnvalue_7 (`GComponent.GetChild` (`self.ListItem`) "t3" "/Script/FairyGUI.GObject"))
  (bind _returnvalue_8 (`GComponent.GetChild` (`self.ListItem`) "cb" "/Script/FairyGUI.GButton"))
  (bind _returnvalue_9 (`GComponent.GetChild` (`self.ListItem`) "t1" "/Script/FairyGUI.GObject"))
  (bind _returnvalue_10 (`GComponent.GetChild` (`self.ListItem`) "mc" "/Script/FairyGUI.GMovieClip"))
  (bind _returnvalue_11 (`GComponent.GetChild` _demoobject_2 "b" null))
  (bind _returnvalue_12 (`GComponent.GetChild` _demoobject_2 "d" null))
  (bind _returnvalue_13 (`GComponent.GetChild` _demoobject_2 "n7" null))
  (bind _returnvalue_14 (`GComponent.GetChild` (`self.DemoObject`) "n25" "/Script/FairyGUI.GButton"))
  (bind _returnvalue_15 (`GComponent.GetChild` (`self.DemoObject`) "n12" "/Script/FairyGUI.GRichTextField"))
  (bind _returnvalue_16 (`GComponent.GetChild` _demoobject_3 "n22" "/Script/FairyGUI.GComponent"))
  (bind _returnvalue_17 (`GComponent.GetChild` (`self.DemoObject`) "n34" "/Script/FairyGUI.GButton"))
  (bind _returnvalue_18 (`GComponent.GetChild` _returnvalue_16 "n0" null))
  (bind _returnvalue_19 (`GObject.CastTo` (`GComponent.GetChild` (`self.DemoObject`) "trapezoid" "/Script/FairyGUI.GGraph") "/Script/FairyGUI.GGraph"))
  (switch `string` (`self.DemoName`)
    (:`Demo_Popup`
      (`GComponent.OnClickChild` _demoobject_6 "n0" (`|CreateDelegate` :!event `Event PopupMenu`))
      (`GComponent.OnClickChild` _demoobject_6 "n1" (`|CreateDelegate` :!event `Event PopupPanel`)))
    (:`Demo_Window`
      (`GComponent.OnClickChild` _demoobject_5 "n0" (delegate `Event ShowWindow1`))
      (`GComponent.OnClickChild` _demoobject_5 "n1" (delegate `Event ShowWindow2`)))
    (:`Demo_ProgressBar`
      (for _index (range (`GComponent.NumChildren` _demoobject_4)) :!label _label
        (bind _asgprogress_bar (cast `GProgressBar` (`GComponent.GetChildAt` _demoobject_4 _index null)))
        (bind _returnvalue_20 (+ (`GProgressBar.GetValue` _asgprogress_bar) 1.0))
        (if (< _returnvalue_20 (`GProgressBar.GetMax` _asgprogress_bar))
          (`GProgressBar.SetValue` _asgprogress_bar _returnvalue_20)
          (else
            (`GProgressBar.SetValue` _asgprogress_bar 0.0)))))
    (:`Demo_Depth`
      (`GComponent.OnClickChild` _demoobject_3 "btn0" (`|CreateDelegate` :!event `Event AddChild`))
      (`GComponent.OnClickChild` _demoobject_3 "btn1" (`|CreateDelegate` :!event `Event AddChildWithDepth`))
      (set `self.FixedObj` _returnvalue_18)
      (`GObject.SetSortingOrder` _returnvalue_18 100)
      (`GObject.SetDraggable` _returnvalue_18 true)
      (set `self.AddChildPos` (`GObject.GetPosition` _returnvalue_18))
      (`GComponent.RemoveChildren` _returnvalue_16 0 -1)
      (`GComponent.AddChild` _returnvalue_16 (`self.FixedObj`)))
    (:`Demo_Drag&Drop`
      (`GObject.SetDraggable` (`GComponent.GetChild` _demoobject_2 "a" null) true)
      (`GObject.SetDraggable` _returnvalue_11 true)
      (add `GObject.OnDragStart` _returnvalue_11 (delegate `OnDragStart_Event_0`))
      (add `GComponent.OnDrop` (`GComponent.GetChild` _demoobject_2 "c" "/Script/FairyGUI.GComponent") (delegate `OnDrop_Event_0`))
      (`GObject.SetDraggable` _returnvalue_12 true)
      (bind _returnvalue_21 (`GObject.LocalToRootRect` _returnvalue_13 (`KismetMathLibrary.MakeBox2D` (0.0 0.0) (`GObject.GetSize` _returnvalue_13))))
      (`GObject.SetDragBounds` _returnvalue_12 _returnvalue_21))
    (:`Demo_Text`
      (`/Engine/EditorBlueprintResources/StandardMacros.IsValid` _returnvalue_14
        (:`Is Valid`
          (add `GObject.OnClick` _returnvalue_14 (delegate `OnClick_事件_0`))
          (`/Engine/EditorBlueprintResources/StandardMacros.IsValid` _returnvalue_15
            (:`Is Valid`
              (add `GRichTextField.OnHtmlLinkClick` _returnvalue_15 (delegate `OnHtmlLinkClick_事件`)))))))
    (:`Demo_Graph`
      (`/Engine/EditorBlueprintResources/StandardMacros.IsValid` _returnvalue_19
        (:`Is Valid`
          (bind _returnvalue_22 (`UIPackage.GetImageItem` "Basics" "change"))
          (`/Engine/EditorBlueprintResources/StandardMacros.IsValid` _returnvalue_22
            (:`Is Valid`
              (`GGraph.SetType` _returnvalue_19 "Polygon")
              (`GGraph.SetUsePercentPositions` _returnvalue_19 true)
              (`GGraph.SetTexture` _returnvalue_19 _returnvalue_22)
              (`GGraph.SetPolygonPoints` _returnvalue_19 (`|MakeArray` (0.0 1.0) (0.3 0.0) (0.7 0.0) (1.0 1.0) :!type "Vector2D Structure"))
              (`GGraph.SetTexcoords` _returnvalue_19 (`|MakeArray` (0.0 1.0) (0.0 0.0) (1.0 0.0) (1.0 1.0) :!type "Vector2D Structure")))))))
    (:`Demo_Button`
      (`/Engine/EditorBlueprintResources/StandardMacros.IsValid` _returnvalue_17
        (:`Is Valid`
          (add `GObject.OnClick` _returnvalue_17 (delegate `OnClick_事件`)))))
    (:`Demo_Grid`
      (`/Engine/EditorBlueprintResources/StandardMacros.IsValid` _returnvalue_2
        (:`Is Valid`
          (`GList.RemoveChildrenToPool` _returnvalue_2 0 -1)
          (set `self.LoopIndex` 0)
          (bind _enumvalue (foreach `EObjectType` false)
            (:`LoopBody`
              (bind _returnvalue_23 (`GList.AddItemFromPool` _returnvalue_2 ""))
              (bind _returnvalue_24 (`GObject.CastTo` _returnvalue_23 "/Script/FairyGUI.GComponent"))
              (`/Engine/EditorBlueprintResources/StandardMacros.IsValid` _returnvalue_24
                (:`Is Valid`
                  (set `self.ListItem` _returnvalue_24)
                  (`/Engine/EditorBlueprintResources/StandardMacros.IsValid` _returnvalue_5
                    (:`Is Valid`
                      (`GObject.SetText` _returnvalue_5 (`KismetTextLibrary.Conv_IntToText` (+ (`self.LoopIndex`) 1)))
                      (`/Engine/EditorBlueprintResources/StandardMacros.IsValid` _returnvalue_6
                        (:`Is Valid`
                          (`GObject.SetText` _returnvalue_6 (`KismetTextLibrary.Conv_StringToText` (`|GetEnumeratorNameAsString` _enumvalue)))
                          (`/Engine/EditorBlueprintResources/StandardMacros.IsValid` _returnvalue_3
                            (:`Is Valid`
                              (`GObject.SetColor` _returnvalue_3 (`KismetMathLibrary.Conv_LinearColorToColor` (`KismetArrayLibrary.Array_Random` (`self.Colors`))))
                              (`/Engine/EditorBlueprintResources/StandardMacros.IsValid` _returnvalue_4
                                (:`Is Valid`
                                  (`GProgressBar.SetValue` _returnvalue_4 (`KismetMathLibrary.Conv_IntToDouble` (/ (* (`KismetMathLibrary.RandomIntegerInRange` 1 4) 100) 3)))
                                  (`/Engine/EditorBlueprintResources/StandardMacros.IncrementInt` (`self.LoopIndex`)))))))))))))
            (:`then`
              (`/Engine/EditorBlueprintResources/StandardMacros.IsValid` _returnvalue
                (:`Is Valid`
                  (`GList.RemoveChildrenToPool` _returnvalue 0 -1)
                  (set `self.LoopIndex` 0)
                  (bind _enumvalue_2 (foreach `EPackageItemType` true)
                    (:`LoopBody`
                      (bind _returnvalue_25 (`GList.AddItemFromPool` _returnvalue ""))
                      (bind _returnvalue_26 (`GObject.CastTo` _returnvalue_25 "/Script/FairyGUI.GComponent"))
                      (`/Engine/EditorBlueprintResources/StandardMacros.IsValid` _returnvalue_26
                        (:`Is Valid`
                          (set `self.ListItem` _returnvalue_26)
                          (`/Engine/EditorBlueprintResources/StandardMacros.IsValid` _returnvalue_8
                            (:`Is Valid`
                              (`GButton.SetSelected` _returnvalue_8 false)
                              (`/Engine/EditorBlueprintResources/StandardMacros.IsValid` _returnvalue_9
                                (:`Is Valid`
                                  (`GObject.SetText` _returnvalue_9 (`KismetTextLibrary.Conv_StringToText` (`|GetEnumeratorNameAsString` _enumvalue_2)))
                                  (`/Engine/EditorBlueprintResources/StandardMacros.IsValid` _returnvalue_10
                                    (:`Is Valid`
                                      (`GMovieClip.SetPlaying` _returnvalue_10 (== (mod (`self.LoopIndex`) 2) 0))
                                      (`/Engine/EditorBlueprintResources/StandardMacros.IsValid` _returnvalue_7
                                        (:`Is Valid`
                                          (`GObject.SetText` _returnvalue_7 (`KismetTextLibrary.Conv_IntToText` (`KismetMathLibrary.RandomIntegerInRange` 0 10000)))
                                          (`/Engine/EditorBlueprintResources/StandardMacros.IncrementInt` (`self.LoopIndex`)))))))))))))))))))))))

(event `Event ShowWindow1`
  (params (EventContext :type "EventContext Object Reference"))
  (bind _window1 (`self.Window1`))
  (`/Engine/EditorBlueprintResources/StandardMacros.IsValid` _window1
    (:`Is Valid`
      _)
    (:`Is Not Valid`
      (bind _returnvalue (`GWindow.CreateWindow` "Basics" "WindowA"))
      (bind _output_get (set `self.Window1` _returnvalue))
      (`GObject.Center` _output_get false)
      (set `GWindow.ShownCallback` (delegate `Event Window1 OnShown`) _output_get)))
  (`GWindow.Show` _window1))

(event `Event ShowWindow2`
  (params (EventContext :type "EventContext Object Reference"))
  (bind _window2 (`self.Window2`))
  (`/Engine/EditorBlueprintResources/StandardMacros.IsValid` _window2
    (:`Is Valid`
      _)
    (:`Is Not Valid`
      (bind _returnvalue (`GWindow.CreateWindow` "Basics" "WindowB"))
      (bind _output_get (set `self.Window2` _returnvalue))
      (`GObject.Center` _output_get false)
      (set `GWindow.ShownCallback` (delegate `Event Window2 OnShown`) _output_get)))
  (`GWindow.Show` _window2))

(event `Event Window1 OnShown`
  (params (Window :type "GWindow Object Reference"))
  (bind _returnvalue (`GComponent.GetChild` (`GWindow.GetContentPane` (stale `Event ShowWindow1` _output_get)) "n6" "/Script/FairyGUI.GList"))
  (`GList.RemoveChildrenToPool` _returnvalue 0 -1)
  (for _index (range 6)
    (bind _returnvalue_2 (`GList.AddItemFromPool` _returnvalue ""))
    (`GObject.SetText` _returnvalue_2 (`KismetTextLibrary.Conv_StringToText` (`KismetStringLibrary.Conv_IntToString` _index)))
    (`GObject.SetIcon` _returnvalue_2 "ui://Basics/r4")))

(event `Event Window2 OnShown`
  (params (Window :type "GWindow Object Reference"))
  (`Transition.Play` :`self` (`GComponent.GetTransition` (`GWindow.GetContentPane` (stale `Event ShowWindow2` _output_get)) "t1")))

(event `Event AddChild`
  (params (EventContext :type "EventContext Object Reference"))
  (bind _returnvalue (`|GenericCreateObject` self "/Script/FairyGUI.GGraph"))
  (`GObject.SetSize` _returnvalue (`KismetMathLibrary.MakeVector2D` 150.0 150.0) false)
  (bind _output_get (set `self.AddChildPos` (+ (`self.AddChildPos`) (10.0 10.0))))
  (`GObject.SetPosition` _returnvalue _output_get)
  (`GGraph.DrawRect` _returnvalue 1.0 (make `Color` 0 0 0 255) (make `Color` 0 0 255 255))
  (`GObject.SetParent` _returnvalue (`GComponent.GetChild` (`self.DemoObject`) "n22" "/Script/FairyGUI.GComponent")))

(event `Event AddChildWithDepth`
  (params (EventContext :type "EventContext Object Reference"))
  (bind _returnvalue (`|GenericCreateObject` self "/Script/FairyGUI.GGraph"))
  (`GObject.SetSize` _returnvalue (`KismetMathLibrary.MakeVector2D` 150.0 150.0) false)
  (bind _output_get (set `self.AddChildPos` (+ (`self.AddChildPos`) (-10.0 -10.0))))
  (`GObject.SetPosition` _returnvalue _output_get)
  (`GObject.SetSortingOrder` _returnvalue 200)
  (`GGraph.DrawRect` _returnvalue 1.0 (make `Color` 0 0 0 255) (make `Color` 0 255 0 255))
  (`GObject.SetParent` _returnvalue (`GComponent.GetChild` (`self.DemoObject`) "n22" "/Script/FairyGUI.GComponent")))

(event `OnDragStart_Event_0`
  (params (EventContext :type "EventContext Object Reference"))
  (bind _returnvalue (`GObject.GetIcon` (`EventContext.GetSender` EventContext)))
  (`EventContext.PreventDefault` EventContext)
  (bind _returnvalue_2 (`FairyBlueprintLibrary.SetVariantString` (make `NVariant`) _returnvalue))
  (`DragDropManager.StartDrag` (`FairyApplication.GetDragDropManager` (`FairyApplication.Get`)) _returnvalue _returnvalue_2 -1 -1))

(event `OnDrop_Event_0`
  (params (EventContext :type "EventContext Object Reference"))
  (`GObject.SetIcon` (`EventContext.GetSender` EventContext) (`FairyBlueprintLibrary.GetVariantAsString` (`EventContext.GetData` EventContext))))

(event `OnClick_事件_0`
  (params (EventContext :type "EventContext Object Reference"))
  (bind _demoobject (`self.DemoObject`))
  (`GObject.SetText` (`GComponent.GetChild` _demoobject "n24" null) (`GObject.GetText` (`GComponent.GetChild` _demoobject "n22" null))))

(event `OnHtmlLinkClick_事件`
  (params (EventContext :type "EventContext Object Reference"))
  (bind _returnvalue (`GObject.CastTo` (`EventContext.GetSender` EventContext) "/Script/FairyGUI.GRichTextField"))
  (`/Engine/EditorBlueprintResources/StandardMacros.IsValid` _returnvalue
    (:`Is Valid`
      (`GObject.SetText` _returnvalue (`KismetTextLibrary.Conv_StringToText` (`KismetStringLibrary.Concat_StrStr` "[img]ui://Basics/pet[/img][color=#FF0000]You click the link[/color]：" (`FairyBlueprintLibrary.GetVariantAsString` (`EventContext.GetData` EventContext))))))))

(event `self.OnDemoTick`
  (bind (_value _returnvalue) (`BlueprintMapLibrary.Map_Find` (`self.DemoObjects`) "Demo_ProgressBar"))
  (if _returnvalue
    (if (`GObject.OnStage` _value)
      (goto _label))))

(event `OnClick_事件`
  (params (EventContext :type "EventContext Object Reference"))
  (`KismetSystemLibrary.PrintString` "click button" false))