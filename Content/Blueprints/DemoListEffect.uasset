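; FairyGUI demo Blueprint that shows a fullscreen mail list whose visible items play a staggered effect.
; On start it loads the ListEffect package, binds the MailItem extension class and fills the pooled list with placeholder mails in alternating read and fetched states.
; After updating list bounds, it triggers each item's effect with increasing delay, stopping at the first item out of view.
; On end it removes the package.
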(event `self.OnDemoStart`
  (bind _list (`self.List`))
  (bind _delay (`self.Delay`))
  (`UIObjectFactory.SetExtensionWithClass` "ui://ListEffect/mailItem" "/Game/Blueprints/MailItem.MailItem_C")
  (`UIPackage.AddPackage` "/Game/UI/ListEffect.ListEffect")
  (bind _returnvalue (`UIPackage.CreateObject` "ListEffect" "Main" "/Script/FairyGUI.GComponent"))
  (bind _output_get (set `self.MainView` _returnvalue))
  (`GObject.SetParent` _output_get (`GRoot.Get`))
  (`GObject.MakeFullScreen` _output_get false)
  (bind _output_get_2 (set `self.List` (`GComponent.GetChild` _output_get "mailList" "/Script/FairyGUI.GList")))
  (for _index (range 10)
    (bind _returnvalue_2 (`GList.AddItemFromPool` _output_get_2 ""))
    (bind _returnvalue_3 (`GObject.CastTo` _returnvalue_2 "/Game/Blueprints/MailItem.MailItem_C"))
    (`/Game/Blueprints/MailItem.SetFectched` _returnvalue_3 (== (mod _index 3) 0))
    (`/Game/Blueprints/MailItem.SetRead` _returnvalue_3 (== (mod _index 2) 0))
    (`/Game/Blueprints/MailItem.SetTime` _returnvalue_3 "5 Nov 2015 16:24:33")
    (`GButton.SetTitle` _returnvalue_3 "Mail title here"))
  (`GComponent.EnsureBoundsCorrect` _output_get_2)
  (set `self.Delay` 0.5)
  (for _index_2 (range 10)
    (bind _returnvalue_4 (`GComponent.GetChildAt` _list _index_2 "/Game/Blueprints/MailItem.MailItem_C"))
    (if (`GComponent.IsChildInView` _list _returnvalue_4)
      (`/Game/Blueprints/MailItem.PlayEffect` _returnvalue_4 _delay)
      (set `self.Delay` (+ _delay 0.2))
      (else
        (break)))))

(event `self.OnDemoEnd`
  (`UIPackage.RemovePackage` "ListEffect"))