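; FairyGUI demo of a virtualized mail list that shows a thousand items through a virtual GList.
; On start it loads the VirtualList package, registers MailItem as the item class and builds the Main view.
; An item renderer fills each row's fetched and read states, time and title from its index.
; Three buttons select and scroll to a middle item or jump to top or bottom; demo end unloads the package.
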(event `self.OnDemoStart`
  (bind _returnvalue (`GRoot.Get`))
  (bind _mainview (`self.MainView`))
  (`UIObjectFactory.SetExtensionWithClass` "ui://VirtualList/MailItem" "/Game/Blueprints/MailItem.MailItem_C")
  (`UIPackage.AddPackage` "/Game/UI/VirtualList.VirtualList")
  (bind _returnvalue_2 (`UIPackage.CreateObject` "VirtualList" "Main" "/Script/FairyGUI.GComponent"))
  (bind _output_get (set `self.MainView` _returnvalue_2))
  (`GObject.SetParent` _output_get _returnvalue)
  (`GObject.SetSize` _output_get (`GObject.GetSize` _returnvalue) false)
  (bind _output_get_2 (set `self.List` (`GComponent.GetChild` _output_get "mailList" "/Script/FairyGUI.GList")))
  (`GList.SetItemRenderer` _output_get_2 (`|CreateDelegate` :!event `ListItemRenderer`))
  (`GList.SetVirtual` _output_get_2)
  (`GList.SetNumItems` _output_get_2 1000)
  (`GComponent.OnClickChild` _mainview "n6" (`|CreateDelegate` :!event `OnClick_Event_0`))
  (`GComponent.OnClickChild` _mainview "n7" (`|CreateDelegate` :!event `OnClick_Event_1`))
  (`GComponent.OnClickChild` _mainview "n8" (`|CreateDelegate` :!event `OnClick_Event_2`)))

(event `self.OnDemoEnd`
  (`UIPackage.RemovePackage` "VirtualList"))

(event `OnClick_Event_0`
  (params (EventContext :type "EventContext Object Reference"))
  (`GList.AddSelection` (`self.List`) 500 true))

(event `OnClick_Event_1`
  (params (EventContext :type "EventContext Object Reference"))
  (`ScrollPane.ScrollTop` (`GComponent.GetScrollPane` (`self.List`)) false))

(event `OnClick_Event_2`
  (params (EventContext :type "EventContext Object Reference"))
  (`ScrollPane.ScrollBottom` (`GComponent.GetScrollPane` (`self.List`)) false))

(event `ListItemRenderer`
  (params (Index :type Integer) (Obj :type "GObject Object Reference"))
  (bind _returnvalue (`GObject.CastTo` Obj "/Game/Blueprints/MailItem.MailItem_C"))
  (`/Game/Blueprints/MailItem.SetFectched` _returnvalue (== (mod Index 3) 0))
  (`/Game/Blueprints/MailItem.SetRead` _returnvalue (== (mod Index 2) 0))
  (`/Game/Blueprints/MailItem.SetTime` _returnvalue "2 Mar 2021 11:26:33")
  (`GObject.SetText` _returnvalue (`KismetStringLibrary.Concat_StrStr` (`KismetStringLibrary.Conv_IntToString` Index) " Mail title here")))